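; ZombieCharacterBP is a zombie character that switches its AI state and network dormancy together.
; Its ChangeEnum event runs only on the server and maps the incoming value to one of two EState values on the Blackboard's State key.
; The first state puts replication into DormantAll and the second wakes it, with a NetAwake flag preventing redundant dormancy changes.
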(event `self.ChangeEnum`
  (params (value :type Integer))
  (bind _returnvalue (`AIBlueprintHelperLibrary.GetBlackboard` null))
  (if (`KismetSystemLibrary.IsServer`)
    (switch `int` value
      (:`0`
        (`BlackboardComponent.SetValueAsEnum` _returnvalue "State" (enumliteral `/Game/Blueprints/EState` "NewEnumerator0"))
        (if (`self.bNetAwake`)
          (`self.SetNetDormancy` "DORM_DormantAll")
          (set `self.bNetAwake` false)))
      (:`1`
        (`BlackboardComponent.SetValueAsEnum` _returnvalue "State" (enumliteral `/Game/Blueprints/EState` "NewEnumerator1"))
        (if (not (`self.bNetAwake`))
          (`self.SetNetDormancy` "DORM_Awake")
          (set `self.bNetAwake` true))))))

(fn `UserConstructionScript`)