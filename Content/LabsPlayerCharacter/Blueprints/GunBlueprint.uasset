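; GunBlueprint is a gun that tracks magazine ammo and the cooldown between shots for the player character.
; BeginPlay fills the magazine, and Tick counts down the shot timer, then re-enables firing once it expires with rounds remaining.
; Fire, which takes a launch direction, and Reload are empty stubs, so nothing here spends rounds or starts the cooldown.
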(event `self.ReceiveBeginPlay`
  (set `self.RoundRemianingInMagazine` (`self.MagazineSize`)))

(event `self.ReceiveTick`
  (params (DeltaSeconds :type "Float (single-precision)"))
  ;[1 1 1] Fire Cooldown
  (if (and (not (`self.bCanFire`)) (> (`self.TimeTillNextShot`) 0.0))
    (set `self.TimeTillNextShot` (- (`self.TimeTillNextShot`) DeltaSeconds))
    (elif (and (<= (`self.TimeTillNextShot`) 0.0) (> (`self.RoundRemianingInMagazine`) 0))
      (set `self.bCanFire` true))))

(fn `Fire`
  (params (LaunchDirection :type "Vector Structure")))

(fn `Reload`)

(fn `UserConstructionScript`)